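; Dynamite pickup that adds one wall explosive to the first-person player character, as long as the count is not above four.
; DynamitePickupEvent checks a Triggered flag and the cap, so the pickup grants only once and stays in place when the player is full.
; On success it plays the fuse sound, hides all components, and destroys itself after a short delay.
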(event `DynamitePickupEvent`
  (if (not (`self.triggered`))
    (bind _asbp_first_person_character (cast `/Game/FirstPerson/Blueprints/BP_FirstPersonCharacter` (`GameplayStatics.GetPlayerCharacter` 0)))
    (bind _wallexplosives (`/Game/FirstPerson/Blueprints/BP_FirstPersonCharacter.WallExplosives` _asbp_first_person_character))
    (if (not (> _wallexplosives 4))
      (set `/Game/FirstPerson/Blueprints/BP_FirstPersonCharacter.WallExplosives` (+ _wallexplosives 1) _asbp_first_person_character)
      (set `self.triggered` true)
      (`AudioComponent.Play` (`self.dynamitefuse`) 0.0)
      (`SceneComponent.SetVisibility` (`self.DefaultSceneRoot`) false true)
      (`KismetSystemLibrary.Delay` 2.5)
      (`self.K2_DestroyActor`))))

(fn `UserConstructionScript`)