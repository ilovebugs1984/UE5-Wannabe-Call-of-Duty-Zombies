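; BP_Zombie_Shambler is a zombie enemy with randomized walk speed that hunts and attacks the player.
; Pawn sensing triggers a chase and attack montage, whose completion checks a collider overlap before damaging and launching the player.
; AI perception stimuli draw it to their location until it has seen the player; a separate Roam event moves it to random nearby points.
; Damage plays a hit reaction or, at zero health, a death animation followed by delayed destruction.
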(event `self.ReceiveBeginPlay`
  (set `CharacterMovementComponent.MaxWalkSpeed` (`KismetMathLibrary.RandomFloatInRange` 170.0 270.0) (`self.CharacterMovement`)))

(event `Roam`
  (`|AIMoveTo` self (`NavigationSystemV1.K2_GetRandomReachablePointInRadius` (`self.K2_GetActorLocation`) 500.0 null null) null))

(event `self.PawnSensing.OnSeePawn`
  (params (Pawn :type "Pawn Object Reference"))
  (if (not (`self.Dead`))
    (set `self.Has Seen Player` true)
    (`|AIMoveTo` self (`self.K2_GetActorLocation` Pawn) Pawn 100.0
      (:`OnSuccess`
        (if (not (`self.Attacking`))
          (set `self.Attacking` true)
          (`|PlayMontage` (`self.Mesh`) "/Game/Blueprints/Mechanics/ZombieAI/ZombieExtra/Zombie_AttackMontage.Zombie_AttackMontage" 1.3
            (:`OnCompleted`
              (if (> (`KismetArrayLibrary.Array_Length` (`PrimitiveComponent.GetOverlappingActors` (`self.AttackCollider`) "/Game/FirstPerson/Blueprints/BP_FirstPersonCharacter.BP_FirstPersonCharacter_C")) 0)
                (bind _asbp_first_person_character (cast `/Game/FirstPerson/Blueprints/BP_FirstPersonCharacter` (`GameplayStatics.GetPlayerCharacter` 0)))
                (`/Game/FirstPerson/Blueprints/BP_FirstPersonCharacter.DamagePlayer` _asbp_first_person_character 50)
                (`self.LaunchCharacter` _asbp_first_person_character (* (`self.K2_GetActorLocation` _asbp_first_person_character) 1.1) false true)
                (set `self.Attacking` false)
                (else
                  (set `self.Attacking` false))))
            (:`OnInterrupted`
              (set `self.Attacking` false))))))))

(event `self.ReceiveAnyDamage`
  (params (Damage :type "Float (single-precision)") (DamageType :type "DamageType Object Reference") (InstigatedBy :type "Controller Object Reference") (DamageCauser :type "Actor Object Reference"))
  (bind _mesh (`self.Mesh`))
  (bind _output_get (set `self.Health` (- (`self.Health`) Damage)))
  (if (<= _output_get 0.0)
    (`SkeletalMeshComponent.PlayAnimation` _mesh "/Game/Blueprints/Animations/Mannequin_UE5/anim_Burst_B.anim_Burst_B" false)
    (set `self.Dead` true)
    (set `CharacterMovementComponent.MaxWalkSpeed` 0.0 (`self.CharacterMovement`))
    (`AudioComponent.Stop` (`self.ZombieSFX_Cue`))
    (`self.SetActorEnableCollision` false)
    (`KismetSystemLibrary.Delay` 15.0)
    (`self.K2_DestroyActor`)
    (else
      (`|PlayMontage` _mesh "/Game/Blueprints/Mechanics/ZombieAI/ZombieExtra/Zombie_Taking_DMG.Zombie_Taking_DMG" 0.7))))

(event `self.AIPerception.OnTargetPerceptionUpdated`
  (params (Actor :type "Actor Object Reference") (Stimulus :type "AIStimulus Structure"))
  (if (not (`self.Has Seen Player`))
    (`|AIMoveTo` self Stimulus_StimulusLocation null)))

(event `self.ZombieSFX_Cue.OnAudioFinished`
  (if (not (`self.Dead`))
    (`AudioComponent.Play` (`self.ZombieSFX_Cue`) 0.0)))

(fn `UserConstructionScript`)