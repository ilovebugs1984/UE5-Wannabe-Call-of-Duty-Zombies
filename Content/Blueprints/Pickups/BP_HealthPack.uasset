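; BP_HealthPack is a health pickup that adds an amount to the first-person player character's health.
; Its HealthPackGained event works only once and only while the player's health is below a fixed threshold, adding the amount without clamping the result.
; On pickup it plays the Medkit sound and hides itself, then destroys the actor when the audio finishes.
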(event `HealthPackGained`
  (if (not (`self.triggered`))
    (bind _asbp_first_person_character (cast `/Game/FirstPerson/Blueprints/BP_FirstPersonCharacter` (`GameplayStatics.GetPlayerCharacter` 0)))
    (if (not (>= (`/Game/FirstPerson/Blueprints/BP_FirstPersonCharacter.HealthInt` _asbp_first_person_character) 125))
      (set `self.triggered` true)
      (set `/Game/FirstPerson/Blueprints/BP_FirstPersonCharacter.HealthInt` (+ (`/Game/FirstPerson/Blueprints/BP_FirstPersonCharacter.HealthInt` _asbp_first_person_character) (`self.Amount`)) _asbp_first_person_character)
      (`AudioComponent.Play` (`self.medkit`) 0.0)
      (`SceneComponent.SetVisibility` (`self.DefaultSceneRoot`) false true))))

(event `self.medkit.OnAudioFinished`
  (`self.K2_DestroyActor`))

(fn `UserConstructionScript`)