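; Ammo pack pickup that adds pistol ammo to the first-person player character, up to a fixed cap.
; AddAmmunition runs once behind a Triggered flag, which is set before the cap check, so a call at full ammo still uses up the trigger.
; On a successful pickup it plays the Ammobox sound and hides the actor's components.
; The actor destroys itself when that audio finishes.
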(event `AddAmmunition`
  (if (not (`self.triggered`))
    (set `self.triggered` true)
    (bind _asbp_first_person_character (cast `/Game/FirstPerson/Blueprints/BP_FirstPersonCharacter` (`GameplayStatics.GetPlayerCharacter` 0)))
    (bind _pistol_ammo (`/Game/FirstPerson/Blueprints/BP_FirstPersonCharacter.Pistol_Ammo` _asbp_first_person_character))
    (if (not (>= _pistol_ammo 49))
      (bind _output_get (set `/Game/FirstPerson/Blueprints/BP_FirstPersonCharacter.Pistol_Ammo` (+ _pistol_ammo 7) _asbp_first_person_character))
      (if (>= _output_get 49)
        (set `/Game/FirstPerson/Blueprints/BP_FirstPersonCharacter.Pistol_Ammo` 49 _asbp_first_person_character))
      (`AudioComponent.Play` (`self.ammobox`) 0.0)
      (`SceneComponent.SetVisibility` (`self.DefaultSceneRoot`) false true))))

(event `self.ammobox.OnAudioFinished`
  (`self.K2_DestroyActor`))

(fn `UserConstructionScript`)