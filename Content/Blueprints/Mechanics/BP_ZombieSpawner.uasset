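; Zombie spawner that links to an overlapping BP_Window and spawns zombies there once that window enables them.
; Tick drives a delayed spawn, skipped while the window is barricaded, picking a random class from the active zombie array.
; After each spawn, Threat thresholds add Goon and Sprinter types to that array once each.
; Hell Mode randomizes the spawn delay at BeginPlay.
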(event `self.ReceiveBeginPlay`
  (if (`self.HellMode`)
    (set `self.DelayPerZombieSpawn` (`KismetMathLibrary.RandomFloatInRange` 5.0 10.0)))
  ; dont overlap windows
  (if (`self.Runner_Added`)
    (`KismetArrayLibrary.Array_Add` (`self.ActiveZombieArray`) "/Game/Blueprints/Mechanics/ZombieAI/BP_Zombie_Sprinter.BP_Zombie_Sprinter_C"))
  (for _array_element (`self.GetOverlappingActors` "/Game/Blueprints/Mechanics/BP_Window.BP_Window_C")
    (set `self.Window` _array_element)
    (break)))

(event `self.ReceiveTick`
  (params (DeltaSeconds :type "Float (single-precision)"))
  (bind _activezombiearray (`self.ActiveZombieArray`))
  (bind _window (`self.Window`))
  (bind (_returnvalue_location _returnvalue_rotation) (`KismetMathLibrary.BreakTransform` (`SceneComponent.K2_GetComponentToWorld` (`self.spawner`))))
  (if (`self.ZombiesActive`)
    (if (`self.Dont_Spawn_Multiple`)
      (`/Game/Blueprints/Mechanics/BP_Window.CheckIfBarricade` _window))
    (if (`/Game/Blueprints/Mechanics/BP_Window.Barricaded` _window)
      (`KismetSystemLibrary.PrintString` "window is barricaded")
      (else
        (set `self.Dont_Spawn_Multiple` true)
        (`KismetSystemLibrary.Delay` (`self.DelayPerZombieSpawn`))
        (if (`/Game/Blueprints/Mechanics/BP_Window.Barricaded` (`self.Window`))
          (`KismetSystemLibrary.PrintString` "Hello")
          (else
            (`|SpawnActorFromClass` (`|GetArrayItem` _activezombiearray (`KismetMathLibrary.RandomIntegerInRange` 0 (`KismetArrayLibrary.Array_Length` _activezombiearray))) (`KismetMathLibrary.MakeTransform` _returnvalue_location _returnvalue_rotation) "AdjustIfPossibleButAlwaysSpawn" "MultiplyWithRoot" null null)
            (set `self.Dont_Spawn_Multiple` false)
            (`self.ThreatLevelAddZombieType`)))))
    (elif (`/Game/Blueprints/Mechanics/BP_Window.ZombiesEnabled` (`self.Window`))
      (set `self.ZombiesActive` true)
      (`KismetSystemLibrary.PrintString` "zombies active"))))

(event `ThreatLevelAddZombieType`
  (`self.AttemptRunnerAdd`)
  (`self.AttemptGoonAdd`))

(event `AttemptGoonAdd`
  (if (>= (`self.Threat`) 15)
    (if (not (`self.Goon_Added`))
      (`KismetArrayLibrary.Array_Add` (`self.ActiveZombieArray`) "/Game/Blueprints/Mechanics/ZombieAI/BP_Zombie_Goon.BP_Zombie_Goon_C")
      (set `self.Goon_Added` true)
      (`KismetSystemLibrary.PrintString` "GOONS ADDED TO SPAWN ARRAYS"))))

(event `AttemptRunnerAdd`
  (if (>= (`self.Threat`) 40)
    (if (not (`self.Runner_Added`))
      (`KismetArrayLibrary.Array_Add` (`self.ActiveZombieArray`) "/Game/Blueprints/Mechanics/ZombieAI/BP_Zombie_Sprinter.BP_Zombie_Sprinter_C")
      (set `self.Runner_Added` true)
      (`KismetSystemLibrary.PrintString` "RUNNERS ADDED TO SPAWN ARRAYS"))))

(fn `UserConstructionScript`)