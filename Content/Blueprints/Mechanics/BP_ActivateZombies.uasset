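; BP_ActivateZombies is a trigger box that switches on the zombie threat when the first-person character walks into it.
; After a configurable delay, it finds every BP_ZombieSpawner and BP_Window in the level and sets their active flags.
; It then marks all BP_ActivateZombies instances as activated, plays the Tankzombiespotted component and destroys itself after a short wait.
; The Activated flag is set only after the first delay, so other triggers stay live until then.
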(event `self.Box.OnComponentBeginOverlap`
  (params (OverlappedComponent :type "PrimitiveComponent Object Reference") (OtherActor :type "Actor Object Reference") (OtherComp :type "PrimitiveComponent Object Reference") (OtherBodyIndex :type Integer) (bFromSweep :type Boolean) (SweepResult :type "HitResult Structure (by ref)"))
  (if (not (`self.activated`))
    (cast `/Game/FirstPerson/Blueprints/BP_FirstPersonCharacter` OtherActor)
    (bind _outactors (`GameplayStatics.GetAllActorsOfClass` "/Game/Blueprints/Mechanics/BP_ZombieSpawner.BP_ZombieSpawner_C"))
    (`KismetSystemLibrary.Delay` (`self.timer till active`))
    (for _array_element _outactors
      (set `/Game/Blueprints/Mechanics/BP_ZombieSpawner.ZombiesActive` true _array_element))
    (bind _outactors_2 (`GameplayStatics.GetAllActorsOfClass` "/Game/Blueprints/Mechanics/BP_Window.BP_Window_C"))
    (for _array_element_2 _outactors_2
      (set `/Game/Blueprints/Mechanics/BP_Window.ZombiesEnabled` true _array_element_2))
    (set `self.activated` true)
    (bind _outactors_3 (`GameplayStatics.GetAllActorsOfClass` "BP_ActivateZombies_C"))
    (for _array_element_3 _outactors_3
      (set `/Game/Blueprints/Mechanics/BP_ActivateZombies.activated` true _array_element_3))
    (`AudioComponent.Play` (`self.tankzombiespotted`) 0.0)
    (`KismetSystemLibrary.Delay` 7.0)
    (`self.K2_DestroyActor`)))

(fn `UserConstructionScript`)