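; BP_Window is a window that the player can board up with up to three barricades and that loses them over time while zombies are enabled.
; Player_Barricade_Event spends one of the first-person character's Barricades to show the first inactive board.
; A Delay on Tick periodically hides the first active board.
; An ActiveBarricades bool array mirrors the mesh visibility and is scanned to update the Barricaded flag.
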(event `self.ReceiveTick`
  (params (DeltaSeconds :type "Float (single-precision)"))
  (if (`self.ZombiesEnabled`)
    (`KismetSystemLibrary.Delay` (`self.BarricadeDestructionTimer`))
    (`self.Remove Visual Barricade`)
    (`self.CheckIfBarricade`)))

(event `self.ReceiveBeginPlay`
  (bind _barricadearray (`self.BarricadeArray`))
  (`KismetArrayLibrary.Array_Add` _barricadearray (`self.Barricade One`))
  (`KismetArrayLibrary.Array_Add` _barricadearray (`self.Barricade Two`))
  (`KismetArrayLibrary.Array_Add` _barricadearray (`self.Barricade Three`)))

(event `Add Visual Barricade`
  (for (_array_element _array_index) (`self.Active Barricades`)
    (if (not _array_element)
      (`SceneComponent.SetVisibility` (`|GetArrayItem` (`self.BarricadeArray`) _array_index) true true)
      (`KismetArrayLibrary.Array_Set` (`self.Active Barricades`) _array_index true)
      (`self.CheckIfBarricade`)
      (break))))

(event `Remove Visual Barricade`
  (for (_array_element _array_index) (`self.Active Barricades`)
    (if _array_element
      (`SceneComponent.SetVisibility` (`|GetArrayItem` (`self.BarricadeArray`) _array_index) false true)
      (`KismetArrayLibrary.Array_Set` (`self.Active Barricades`) _array_index)
      (break))))

(event `CheckIfBarricade`
  (set `self.Barricaded` false)
  (for _array_element (`self.Active Barricades`)
    (if _array_element
      (bind _output_get (set `self.Barricaded` true))
      (`KismetSystemLibrary.PrintString` (`KismetStringLibrary.Conv_BoolToString` _output_get))
      (break))))

(event `Player_Barricade_Event`
  (bind _asbp_first_person_character (cast `/Game/FirstPerson/Blueprints/BP_FirstPersonCharacter` (`GameplayStatics.GetPlayerCharacter` 0)))
  (bind _barricades (`/Game/FirstPerson/Blueprints/BP_FirstPersonCharacter.Barricades` _asbp_first_person_character))
  (if (>= _barricades 1)
    (for _array_element (`self.Active Barricades`)
      (if (not _array_element)
        (`self.Add Visual Barricade`)
        (`self.CheckIfBarricade`)
        (bind _result (`/Engine/EditorBlueprintResources/StandardMacros.DecrementInt` _barricades)
          (:`  `
            (set `/Game/FirstPerson/Blueprints/BP_FirstPersonCharacter.Barricades` _result _asbp_first_person_character)
            (break)))))
    (else
      (`KismetSystemLibrary.PrintString` "why are you doing this"))))

(fn `UserConstructionScript`)