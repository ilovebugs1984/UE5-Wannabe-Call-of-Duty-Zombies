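; BP_SentryGun is an enemy turret that shoots at the first-person player character when it sees them.
; Pawn sensing snaps the actor to face the player, then after a short random delay spawns a BP_Bullet from its arrow's transform.
; Incoming damage reduces an integer health value, and lethal damage spawns an explosion effect and destroys the turret.
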(event `self.PawnSensing.OnSeePawn`
  (params (Pawn :type "Pawn Object Reference"))
  (bind _asbp_first_person_character (cast `/Game/FirstPerson/Blueprints/BP_FirstPersonCharacter` Pawn))
  (`self.K2_SetActorRotation` (`KismetMathLibrary.FindLookAtRotation` (`self.K2_GetActorLocation`) (`self.K2_GetActorLocation` _asbp_first_person_character)))
  (`KismetSystemLibrary.Delay` (`KismetMathLibrary.RandomFloatInRange` 1.0 2.0))
  (`|SpawnActorFromClass` "/Game/Blueprints/BP_Bullet.BP_Bullet_C" (`SceneComponent.K2_GetComponentToWorld` (`self.Arrow`)) "Undefined" "MultiplyWithRoot" null null))

(event `self.ReceiveAnyDamage`
  (params (Damage :type "Float (single-precision)") (DamageType :type "DamageType Object Reference") (InstigatedBy :type "Controller Object Reference") (DamageCauser :type "Actor Object Reference"))
  (bind _returnvalue (- (`self.HealthInt`) Damage))
  (if (<= _returnvalue 0.0)
    (`GameplayStatics.SpawnEmitterAtLocation` "/Game/StarterContent/Particles/P_Explosion.P_Explosion")
    (`self.K2_DestroyActor`)
    (else
      (set `self.HealthInt` (`KismetMathLibrary.FTrunc` _returnvalue))
      (`KismetSystemLibrary.PrintString` "Hello"))))

(fn `UserConstructionScript`)