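; BP_DestructableWall is a wall the player blows up with a carried wall explosive.
; DestroyWall proceeds once, only if the player's capsule overlaps Interact and WallExplosives is at least one, which it then decrements.
; A timed sequence shows the dynamite, plays the fuse and reveals fire, then explodes with sound and particles.
; Collision is disabled and the scene hidden, and the actor is destroyed after a delay so the sound can finish.
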(event `DestroyWall`
  (bind _fuse (`self.Fuse`))
  (if (not (`self.WallDestroyed`))
    (bind _asbp_first_person_character (cast `/Game/FirstPerson/Blueprints/BP_FirstPersonCharacter` (`GameplayStatics.GetPlayerCharacter` 0)))
    (if (`PrimitiveComponent.IsOverlappingComponent` (`Character.CapsuleComponent` _asbp_first_person_character) (`self.interact`))
      (bind _wallexplosives (`/Game/FirstPerson/Blueprints/BP_FirstPersonCharacter.WallExplosives` _asbp_first_person_character))
      (if (>= _wallexplosives 1)
        (bind _result (`/Engine/EditorBlueprintResources/StandardMacros.DecrementInt` _wallexplosives)
          (:`  `
            (set `/Game/FirstPerson/Blueprints/BP_FirstPersonCharacter.WallExplosives` _result _asbp_first_person_character)
            (set `self.WallDestroyed` true)
            (`SceneComponent.SetVisibility` (`self.dynamite`) true true)
            (`AudioComponent.Play` _fuse 0.0)
            (`KismetSystemLibrary.Delay` 1.5)
            (`SceneComponent.SetVisibility` (`self.fire`) true true)
            (`KismetSystemLibrary.Delay` 3.0)
            (`AudioComponent.Stop` _fuse)
            (`AudioComponent.Play` (`self.explosion`) 0.0)
            (`GameplayStatics.SpawnEmitterAtLocation` "/Game/StarterContent/Particles/P_Explosion.P_Explosion" (`SceneComponent.K2_GetComponentLocation` (`self.dynamite`)))
            (`PrimitiveComponent.SetCollisionEnabled` (`self.interact`) "NoCollision")
            (`PrimitiveComponent.SetCollisionEnabled` (`self.fire`) "NoCollision")
            (`PrimitiveComponent.SetCollisionEnabled` (`self.dynamite`) "NoCollision")
            (`PrimitiveComponent.SetCollisionEnabled` (`self.wall`) "NoCollision")
            (`PrimitiveComponent.SetCollisionEnabled` (`self.ParticleSystem`) "NoCollision")
            (`PrimitiveComponent.SetCollisionEnabled` (`self.dynamite1`) "NoCollision")
            (`SceneComponent.SetVisibility` (`self.Scene`) false true)
            ; so sfx plays
            (`KismetSystemLibrary.Delay` 5.0)
            (`self.K2_DestroyActor`)))))))

(fn `UserConstructionScript`)